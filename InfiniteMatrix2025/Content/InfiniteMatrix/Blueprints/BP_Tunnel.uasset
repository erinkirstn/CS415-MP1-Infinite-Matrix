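; BP_Tunnel is a tunnel segment with a rotating holed wall that BP_Player must pass through.
; The trigger zone adds score, has TunnelSpawner spawn another tunnel with the red state, then destroys this segment.
; Wall hits reduce health or, at zero health, show restart, and set IsRed at low health, which Tick applies as a material swap.
; RandomizeWall picks a random hole mesh and roll, but is not called here.
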(event `self.ReceiveTick`
  (params (DeltaSeconds :type "Float (single-precision)"))
  (`SceneComponent.K2_AddLocalRotation` (`self.WallMesh`) (`KismetMathLibrary.MakeRotator` (* DeltaSeconds (`self.RotateSpeed`))) false false)
  (`self.Set Background Color` (`self.isRed`)))

(event `self.TriggerZone.OnComponentBeginOverlap`
  (params (OverlappedComponent :type "PrimitiveComponent Object Reference") (OtherActor :type "Actor Object Reference") (OtherComp :type "PrimitiveComponent Object Reference") (OtherBodyIndex :type Integer) (bFromSweep :type Boolean) (SweepResult :type "HitResult Structure (by ref)"))
  (bind _asbp_player (cast `/Game/InfiniteMatrix/Blueprints/BP_Player` OtherActor))
  (set `/Game/InfiniteMatrix/Blueprints/BP_Player.ScoreVar` (+ (`/Game/InfiniteMatrix/Blueprints/BP_Player.ScoreVar` _asbp_player) 1.0) _asbp_player)
  (bind _coloroutput (`/Game/InfiniteMatrix/Blueprints/BP_TunnelSpawner.SpawnTunnelAtSpawnPoint` (`self.TunnelSpawner`) (`self.isRed`)))
  (bind _output_get (set `self.isRed` _coloroutput))
  (`self.Set Background Color` _output_get)
  (`self.K2_DestroyActor`)
  (`GameplayStatics.PlaySound2D` "/Engine/VREditor/Sounds/UI/Teleport_Mode_Entered.Teleport_Mode_Entered" 1.0 1.0 0.0 null null))

(event `self.WallMesh.OnComponentHit`
  (params (HitComponent :type "PrimitiveComponent Object Reference") (OtherActor :type "Actor Object Reference") (OtherComp :type "PrimitiveComponent Object Reference") (NormalImpulse :type "Vector Structure") (Hit :type "HitResult Structure (by ref)"))
  (bind _asbp_player (cast `/Game/InfiniteMatrix/Blueprints/BP_Player` OtherActor))
  (if (<= (`/Game/InfiniteMatrix/Blueprints/BP_Player.Health` _asbp_player) 0.0)
    (set `/Game/InfiniteMatrix/Blueprints/BP_Player.IsDead` true _asbp_player)
    (`/Game/InfiniteMatrix/Blueprints/BP_Player.DisplayRestart` _asbp_player)
    (else
      (if (<= (`/Game/InfiniteMatrix/Blueprints/BP_Player.Health` _asbp_player) 0.5)
        (set `self.isRed` true)
        (else
          (set `self.isRed` false)))
      (`/Game/InfiniteMatrix/Blueprints/BP_Player.DecreaseHealth` _asbp_player))))

(fn `RandomizeWall`
  (`StaticMeshComponent.SetStaticMesh` (`self.WallMesh`) (select `int` (`KismetMathLibrary.RandomIntegerInRange` 0 3) :`0` "/Game/InfiniteMatrix/Meshes/SM_Hole_01.SM_Hole_01" :`1` "/Game/InfiniteMatrix/Meshes/SM_Hole_02.SM_Hole_02" :`2` "/Game/InfiniteMatrix/Meshes/SM_Hole_03.SM_Hole_03" :`3` "/Game/InfiniteMatrix/Meshes/SM_Hole_04.SM_Hole_04" :!type "StaticMesh Object Reference"))
  (`SceneComponent.K2_AddLocalRotation` (`self.WallMesh`) (`KismetMathLibrary.MakeRotator` (`KismetMathLibrary.RandomFloatInRange` 0.0 360.0)) false false))

(fn `Set Background Color`
  (params (Color :type Boolean))
  (if (`self.isRed`)
    (`PrimitiveComponent.SetMaterial` (`self.StaticMeshComponent`) 0 "/Game/InfiniteMatrix/Materials/MI_Tunnel2.MI_Tunnel2")
    (`PrimitiveComponent.SetMaterial` (`self.WallMesh`) 0 "/Game/InfiniteMatrix/Materials/MI_Hole2.MI_Hole2")
    (else
      (`PrimitiveComponent.SetMaterial` (`self.StaticMeshComponent`) 0 "/Game/InfiniteMatrix/Materials/MI_Tunnel.MI_Tunnel")
      (`PrimitiveComponent.SetMaterial` (`self.WallMesh`) 0 "/Game/InfiniteMatrix/Materials/MI_Hole.MI_Hole"))))

(fn `UserConstructionScript`)